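; Player character for a pottery shop game that carries clay and items between storage, crafting bench, displays and the haggling register.
; BeginPlay creates the UI widgets, including the main menu, and caches game mode, register and save manager references.
; Overlaps set the interact actor and prompt, and its second tag routes Interact to station-specific handlers that check carry state.
; Input also handles movement, item dropping, day start/end and the upgrade screen toggle.
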(event EventBeginPlay
  ;[1 1 1] Set Can Move
  (Variables|Default|SetCanMove false)
  ;[1 1 1] Create Interact Prompt
  (bind _returnvalue (UserInterface|CreateWidget "/Game/UI_Workspace/Blueprints/P_Interact.P_Interact_C"))
  (Variables|Default|SetInteractPrompt _returnvalue)
  ;[1 1 1] Create Inventory Widget
  (bind _returnvalue_2 (UserInterface|CreateWidget "/Game/UI_Workspace/Blueprints/InventoryDisplay.InventoryDisplay_C"))
  (bind _output_get (Variables|Default|SetInventoryDisplayInstance _returnvalue_2))
  (UserInterface|Viewport|AddtoViewport _output_get 0)
  (Variables|Default|SetInventory%20Scroll%20Box (Variables|/Game/UI_Workspace/Blueprints/InventoryDisplay.InventoryDisplay_C|GetInventoryScrollBox (Variables|Default|GetInventoryDisplayInstance)))
  (Widget|RemovefromParent (Variables|Default|GetInventoryDisplayInstance))
  ;[1 1 1] Create Crafting Screen
  (bind _returnvalue_3 (UserInterface|CreateWidget "/Game/UI_Workspace/Blueprints/CraftingScreen.CraftingScreen_C"))
  (Variables|Default|SetCraftingWindowInstance _returnvalue_3)
  ;[1 1 1] Get GameMode Reference
  (bind _outactors (Actor|GetAllActorsOfClass "/Game/Level_Workspace/Blueprints/GM_GameMode.GM_GameMode_C"))
  (for _array_element _outactors
    (bind _asgm_game_mode (Utilities|Casting|CastToGM_GameMode _array_element))
    (Variables|Default|SetGameModeInstance _asgm_game_mode))
  ;[1 1 1] Create Upgrade Menu
  (bind _returnvalue_4 (UserInterface|CreateWidget "/Game/UI_Workspace/Blueprints/UpgradeScreen.UpgradeScreen_C"))
  (bind _output_get_2 (Variables|Default|SetUpgradeScreenReference _returnvalue_4))
  (UserInterface|Viewport|AddtoViewport _output_get_2 0)
  (Widget|RemovefromParent _output_get_2)
  ;[1 1 1] Get Haggling Screen Reference
  (bind _returnvalue_5 (UserInterface|CreateWidget "/Game/UI_Workspace/Blueprints/HagglingScreen.HagglingScreen_C"))
  (bind _output_get_3 (Variables|Default|SetHagglingScreenInstance _returnvalue_5))
  (UserInterface|Viewport|AddtoViewport _output_get_3 0)
  (Widget|RemovefromParent _output_get_3)
  ;[1 1 1] Get Register Object
  (bind _returnvalue_6 (Actor|GetActorOfClass "/Game/Level_Workspace/Blueprints/Actors/BP_Register.BP_Register_C"))
  (Variables|Default|SetRegisterInstance _returnvalue_6)
  ;[1 1 1] Create Main Menu
  (bind _returnvalue_7 (UserInterface|CreateWidget "/Game/UI_Workspace/Blueprints/MainMenu.MainMenu_C"))
  (UserInterface|Viewport|AddtoViewport _returnvalue_7 0)
  (bind _returnvalue_8 (Actor|GetActorOfClass "/Game/Level_Workspace/Blueprints/SaveGameManager.SaveGameManager_C"))
  (Variables|Default|SetSaveGameInstance _returnvalue_8))

(event Collision|EventActorEndOverlap
  (params (OtherActor :type Actor%20Object%20Reference))
  ;[1 1 1] Remove Pick Up Prompt
  (if (Actor|ActorHasTag OtherActor (Variables|TagReferences|GetPromptTag))
    (if (UserInterface|Viewport|IsinViewport (Variables|Default|GetInteractPrompt))
      (Variables|Default|SetCanInteract false)
      (Widget|RemovefromParent (Variables|Default|GetInteractPrompt)))))

(event Collision|EventActorBeginOverlap
  (params (OtherActor :type Actor%20Object%20Reference))
  ;[1 1 1] Display Pick Up Prompt
  (if (Actor|ActorHasTag OtherActor (Variables|TagReferences|GetPromptTag))
    (Variables|Default|SetInteractActor OtherActor)
    (Variables|Default|SetCanInteract true)
    (CallFunction|DisplayPickUpPrompt)))

(event Input|ActionEvents|InputActionStartDay
  (params (Key :type Key%20Structure :default "None"))
  (bind _gamemodeinstance (Variables|Default|GetGameModeInstance))
  ;[1 1 1] Start New Day
  (:Pressed
    (if (Variables|Default|GetHasGameStarted)
      (if (Variables|/Game/Level_Workspace/Blueprints/GM_GameMode.GM_GameMode_C|GetHasDayStarted _gamemodeinstance)
        (Default|FadeScreen _gamemodeinstance)
        (Utilities|FlowControl|Delay 1.5)
        (Default|EndDay _gamemodeinstance)
        (else
          (Default|StartNewDay _gamemodeinstance))))))

(event Input|ActionEvents|InputActionInteract
  (params (Key :type Key%20Structure :default "None"))
  ;[1 1 1] Interact With Objects In Shop
  (:Pressed
    (if (Variables|Default|GetCanInteract)
      (switch name (Utilities|Array|Get(acopy) (Variables|/Script/Engine.Actor|GetTags (Variables|Default|GetInteractActor)) 1)
        (:Crafting
          (CallFunction|InteractwithCrafting))
        (:ShopDisplay
          (CallFunction|InteractwithShopDisplay))
        (:Register
          (CallFunction|InteractwithRegister))
        (:PickUp
          (CallFunction|InteractwithPickUp))
        (:ClayStorage
          (CallFunction|InteractwithClayStorage)))
      (elif (Variables|Default|GetIsInCrafting)
        (CallFunction|CloseCrafting)
        (elif (Variables|Default|GetIsInCashRegister)
          (CallFunction|CloseRegister))))))

(event Input|ActionEvents|InputActionDropItem
  (params (Key :type Key%20Structure :default "None"))
  ;[1 1 1] Drop Carried Item
  (:Pressed
    (if (Variables|Default|GetIsCarrying)
      (CallFunction|DropItem)
      (Variables|Default|SetCarriedItem (Variables|Default|GetNullActor)))))

(event Input|ActionEvents|InputActionToggleInventory
  (params (Key :type Key%20Structure :default "None"))
  ;[1 1 1] Toggle Inventory
  (:Pressed
    (if (Variables|Default|GetHasGameStarted)
      (if (UserInterface|Viewport|IsinViewport (Variables|Default|GetUpgradeScreenReference))
        (Upgrades|CloseUpgradeScreen)
        (Variables|/Script/Engine.PlayerController|SetbShowMouseCursor (Game|GetPlayerController 0) false)
        (else
          (Upgrades|OpenUpgradeScreen)
          (Variables|/Script/Engine.PlayerController|SetbShowMouseCursor (Game|GetPlayerController 0) true))))))

(event Input|AxisEvents|InputAxisMoveForward
  (params (AxisValue :type Float%20%28single-precision%29))
  ;[1 1 1] Movement
  (if (Variables|Default|GetCanMove)
    (Pawn|Input|AddMovementInput (Math|Vector|MakeVector -1.0 0.0 0.0) AxisValue false)))

(event Input|AxisEvents|InputAxisMoveRight
  (params (AxisValue :type Float%20%28single-precision%29))
  ;[1 1 1] Movement
  (if (Variables|Default|GetCanMove)
    (Pawn|Input|AddMovementInput (Math|Vector|MakeVector 0.0 -1.0 0.0) AxisValue false)))

(fn ConstructionScript)

(fn DisplayPickUpPrompt
  (bind _interactprompt (Variables|Default|GetInteractPrompt))
  (if (Variables|Default|GetCanInteract)
    (if (not (UserInterface|Viewport|IsinViewport (Variables|Default|GetInteractPrompt)))
      (UserInterface|Viewport|AddtoViewport _interactprompt 0)
      (switch name (Utilities|Array|Get(acopy) (Variables|/Script/Engine.Actor|GetTags (Variables|Default|GetInteractActor)) 1)
        (:Crafting
          (Variables|/Script/UMG.TextBlock|SetText (Variables|/Game/UI_Workspace/Blueprints/P_Interact.P_Interact_C|GetInteractText (Variables|Default|GetInteractPrompt)) "E To Craft"))
        (:ShopDisplay
          (Variables|/Script/UMG.TextBlock|SetText (Variables|/Game/UI_Workspace/Blueprints/P_Interact.P_Interact_C|GetInteractText (Variables|Default|GetInteractPrompt)) "E To Place"))
        (:Register
          (Variables|/Script/UMG.TextBlock|SetText (Variables|/Game/UI_Workspace/Blueprints/P_Interact.P_Interact_C|GetInteractText (Variables|Default|GetInteractPrompt)) "E To Haggle"))
        (:PickUp
          (Variables|/Script/UMG.TextBlock|SetText (Variables|/Game/UI_Workspace/Blueprints/P_Interact.P_Interact_C|GetInteractText (Variables|Default|GetInteractPrompt)) "E To Pick Up"))))
    (elif (UserInterface|Viewport|IsinViewport (Variables|Default|GetInteractPrompt))
      (Widget|RemovefromParent _interactprompt))))

(fn AddItemtoInventory
  (params (Item :type Inventory%20Item%20Struct%20Structure%20%28by%20ref%29))
  (Utilities|Array|Add (Variables|Default|GetInventoryContents) Item))

(fn RemoveItemfromInventory
  (params (Item :type Inventory%20Item%20Struct%20Structure%20%28by%20ref%29))
  (Utilities|Array|RemoveItem (Variables|Default|GetInventoryContents) Item))

(fn UpdateInventoryDisplay
  (Widget|Panel|ClearChildren (Variables|Default|GetInventory%20Scroll%20Box))
  (for _array_element (Variables|Default|GetInventoryContents)
    (LocalVariables|SetInventoryItemStruct _array_element)
    (bind _returnvalue (UserInterface|CreateWidget "/Game/UI_Workspace/Blueprints/InventoryButton.InventoryButton_C"))
    (Variables|/Game/UI_Workspace/Blueprints/InventoryButton.InventoryButton_C|SetItemStruct _returnvalue (LocalVariables|GetInventoryItemStruct))
    (Widget|Panel|AddChild (Variables|Default|GetInventory%20Scroll%20Box) _returnvalue)))

(fn OpenInventory
  (CallFunction|UpdateInventoryDisplay)
  (UserInterface|Viewport|AddtoViewport (Variables|Default|GetInventoryDisplayInstance) 0))

(fn CloseInventory
  (Widget|RemovefromParent (Variables|Default|GetInventoryDisplayInstance)))

(fn CloseCrafting
  (Variables|Default|SetIsInCrafting false)
  (Widget|RemovefromParent (Variables|Default|GetCraftingWindowInstance))
  (Variables|/Script/Engine.PlayerController|SetbShowMouseCursor (Game|GetPlayerController 0) false)
  (Variables|Default|SetCanMove true)
  (Variables|Default|SetCanInteract true))

(fn OpenCraftingUI
  (bind _craftingwindowinstance (Variables|Default|GetCraftingWindowInstance))
  (Variables|Default|SetIsInCrafting true)
  (UserInterface|Viewport|AddtoViewport _craftingwindowinstance 0)
  (Variables|/Script/Engine.PlayerController|SetbShowMouseCursor (Game|GetPlayerController 0) true)
  (Variables|Default|SetCanMove false)
  (Variables|Default|SetCanInteract false)
  (Input|SetInputModeGameandUI (Game|GetPlayerController 0) _craftingwindowinstance "DoNotLock" true false))

(fn PlaceinShopDisplay
  (Variables|Default|SetIsCarrying false)
  (Transformation|DetachFromActor (Variables|Default|GetCarriedItem) "KeepWorld" "KeepWorld" "KeepWorld")
  (bind _output_get (Variables|Default|SetItemDisplayPosition (Utilities|Array|Get(acopy) (Actor|GetComponentsbyTag (Variables|Default|GetInteractActor) "/Script/Engine.StaticMeshComponent" "ItemPosition"))))
  (Transformation|AttachComponentToComponent (Actor|GetComponentbyClass (Variables|Default|GetCarriedItem) "/Script/Engine.StaticMeshComponent") _output_get "None" "SnapToTarget" "SnapToTarget" "KeepWorld" true)
  (Collision|SetCollisionEnabled (Utilities|Array|Get(acopy) (Actor|GetComponentsbyTag (Variables|Default|GetCarriedItem) "/Script/Engine.BoxComponent" "PickUpCollision")) "NoCollision")
  (bind _asbp_shop_display (Utilities|Casting|CastToBP_ShopDisplay (Variables|Default|GetInteractActor)))
  (Variables|/Game/Level_Workspace/Blueprints/Actors/BP_ShopDisplay.BP_ShopDisplay_C|SetHasItem _asbp_shop_display true)
  (Variables|/Game/Level_Workspace/Blueprints/Actors/BP_ShopDisplay.BP_ShopDisplay_C|SetHeldItem _asbp_shop_display (Variables|Default|GetCarriedItem))
  (Variables|Default|SetCarriedItem (Variables|Default|GetNullActor)))

(fn OpenRegister
  (Variables|Default|SetIsInCashRegister true)
  (Variables|Default|SetCanMove false)
  (UserInterface|Viewport|AddtoViewport (Variables|Default|GetHagglingScreenInstance) 0)
  (Variables|/Script/Engine.PlayerController|SetbShowMouseCursor (Game|GetPlayerController 0) true))

(fn CloseRegister
  (Variables|Default|SetIsInCashRegister false)
  (Variables|Default|SetCanMove true)
  (Widget|RemovefromParent (Variables|Default|GetHagglingScreenInstance))
  (Variables|/Script/Engine.PlayerController|SetbShowMouseCursor (Game|GetPlayerController 0) false))

(fn DropItem
  (bind _carrieditem (Variables|Default|GetCarriedItem))
  (Variables|Default|SetIsCarrying false)
  (Transformation|DetachFromActor _carrieditem "KeepWorld" "KeepWorld" "KeepWorld")
  (if (Actor|ActorHasTag _carrieditem "Clay")
    (Variables|Default|SetHasClay false)
    (Physics|SetSimulatePhysics (Actor|GetComponentbyClass (Variables|Default|GetCarriedItem) "/Script/Engine.StaticMeshComponent") true)
    (else
      (Physics|SetSimulatePhysics (Actor|GetComponentbyClass (Variables|Default|GetCarriedItem) "/Script/Engine.StaticMeshComponent") true)))
  (Collision|SetCollisionEnabled (Utilities|Array|Get(acopy) (Actor|GetComponentsbyTag (Variables|Default|GetCarriedItem) "/Script/Engine.BoxComponent" "PickUpCollision")) "QueryAndPhysics"))

(fn PickUpItem
  (Variables|Default|SetIsCarrying true)
  (bind _output_get (Variables|Default|SetCarriedItem (Variables|Default|GetInteractActor)))
  (if (Actor|ActorHasTag _output_get "Clay")
    (Variables|Default|SetHasClay true)
    (else
      (Transformation|SetWorldScale3D (Actor|GetComponentbyClass (Variables|Default|GetCarriedItem) "/Script/Engine.SceneComponent") "1.000000,1.000000,1.000000")))
  (Physics|SetSimulatePhysics (Actor|GetComponentbyClass (Variables|Default|GetCarriedItem) "/Script/Engine.StaticMeshComponent") false)
  (Collision|SetCollisionEnabled (Utilities|Array|Get(acopy) (Actor|GetComponentsbyTag (Variables|Default|GetCarriedItem) "/Script/Engine.BoxComponent" "PickUpCollision")) "NoCollision")
  (Transformation|AttachComponentToComponent (Actor|GetComponentbyClass (Variables|Default|GetInteractActor) "/Script/Engine.StaticMeshComponent") (Variables|Default|GetItemPos) "None" "SnapToTarget" "SnapToTarget" "KeepWorld" true))

(fn TakefromShopDisplay
  (Variables|Default|SetIsCarrying true)
  (bind _asbp_shop_display (Utilities|Casting|CastToBP_ShopDisplay (Variables|Default|GetInteractActor)))
  (Variables|Default|SetCarriedItem (Variables|/Game/Level_Workspace/Blueprints/Actors/BP_ShopDisplay.BP_ShopDisplay_C|GetHeldItem _asbp_shop_display))
  (Variables|/Game/Level_Workspace/Blueprints/Actors/BP_ShopDisplay.BP_ShopDisplay_C|SetHasItem _asbp_shop_display false)
  (Variables|/Game/Level_Workspace/Blueprints/Actors/BP_ShopDisplay.BP_ShopDisplay_C|SetHeldItem _asbp_shop_display (Variables|Default|GetNullActor))
  (Physics|SetSimulatePhysics (Actor|GetComponentbyClass (Variables|Default|GetCarriedItem) "/Script/Engine.StaticMeshComponent") false)
  (Collision|SetCollisionEnabled (Utilities|Array|Get(acopy) (Actor|GetComponentsbyTag (Variables|Default|GetCarriedItem) "/Script/Engine.BoxComponent" "PickUpCollision")) "NoCollision")
  (Transformation|AttachComponentToComponent (Actor|GetComponentbyClass (Variables|Default|GetCarriedItem) "/Script/Engine.StaticMeshComponent") (Variables|Default|GetItemPos) "None" "SnapToTarget" "SnapToTarget" "KeepWorld" true))

(fn AddClaytoCrafting
  (Variables|Default|SetHasClay false)
  (Variables|Default|SetIsCarrying false)
  (Transformation|DetachFromActor (Variables|Default|GetCarriedItem) "KeepWorld" "KeepWorld" "KeepWorld")
  (bind _output_get (Variables|Default|SetItemDisplayPosition (Utilities|Array|Get(acopy) (Actor|GetComponentsbyTag (Variables|Default|GetInteractActor) "/Script/Engine.StaticMeshComponent" "ItemPosition"))))
  (Transformation|AttachComponentToComponent (Actor|GetComponentbyClass (Variables|Default|GetCarriedItem) "/Script/Engine.StaticMeshComponent") _output_get "None" "SnapToTarget" "SnapToTarget" "KeepWorld" true)
  (Collision|SetCollisionEnabled (Utilities|Array|Get(acopy) (Actor|GetComponentsbyTag (Variables|Default|GetCarriedItem) "/Script/Engine.BoxComponent" "PickUpCollision")) "NoCollision")
  (bind _asbp_crafting_bench (Utilities|Casting|CastToBP_CraftingBench (Variables|Default|GetInteractActor)))
  (Variables|/Game/Level_Workspace/Blueprints/Actors/BP_CraftingBench.BP_CraftingBench_C|SetHasClay _asbp_crafting_bench true)
  (Variables|/Game/Level_Workspace/Blueprints/Actors/BP_CraftingBench.BP_CraftingBench_C|SetHeldItem _asbp_crafting_bench (Variables|Default|GetCarriedItem))
  (Variables|Default|SetCarriedItem (Variables|Default|GetNullActor)))

(fn AddClaytoStorage
  (bind _asbp_clay_storage (Utilities|Casting|CastToBP_ClayStorage (Variables|Default|GetInteractActor)))
  (Math|Integer|IncrementInt (Variables|/Game/Level_Workspace/Blueprints/Actors/BP_ClayStorage.BP_ClayStorage_C|GetClayAmountStored _asbp_clay_storage)))

(fn RemoveClayfromStorage
  (bind _asbp_clay_storage (Utilities|Casting|CastToBP_ClayStorage (Variables|Default|GetInteractActor)))
  (Math|Integer|DecrementInt (Variables|/Game/Level_Workspace/Blueprints/Actors/BP_ClayStorage.BP_ClayStorage_C|GetClayAmountStored _asbp_clay_storage)))

(fn InteractwithCrafting
  (bind _asbp_crafting_bench (Utilities|Casting|CastToBP_CraftingBench (Variables|Default|GetInteractActor)))
  (if (Variables|Default|GetIsCarrying)
    (if (Variables|Default|GetHasClay)
      (if (Variables|/Game/Level_Workspace/Blueprints/Actors/BP_CraftingBench.BP_CraftingBench_C|GetHasClay _asbp_crafting_bench)
        (Development|PrintText "My hands are full" :!label _label)
        (else
          (CallFunction|AddClaytoCrafting)))
      (else
        (goto _label)))
    (elif (Variables|/Game/Level_Workspace/Blueprints/Actors/BP_CraftingBench.BP_CraftingBench_C|GetHasClay _asbp_crafting_bench)
      (CallFunction|OpenCraftingUI)
      (else
        (Development|PrintText "I need clay for this.")))))

(fn InteractwithShopDisplay
  (bind _interactactor (Variables|Default|GetInteractActor))
  (if (Variables|Default|GetIsCarrying)
    (if (Variables|Default|GetHasClay)
      (Development|PrintText "I can´t place this here")
      (else
        (bind _asbp_shop_display (Utilities|Casting|CastToBP_ShopDisplay _interactactor))
        (if (Variables|/Game/Level_Workspace/Blueprints/Actors/BP_ShopDisplay.BP_ShopDisplay_C|GetHasItem _asbp_shop_display)
          (Development|PrintText "This already has an item")
          (else
            (CallFunction|PlaceinShopDisplay)))))
    (else
      (bind _asbp_shop_display_2 (Utilities|Casting|CastToBP_ShopDisplay _interactactor))
      (if (Variables|/Game/Level_Workspace/Blueprints/Actors/BP_ShopDisplay.BP_ShopDisplay_C|GetHasItem _asbp_shop_display_2)
        (CallFunction|TakefromShopDisplay)
        (else
          (Development|PrintText "I need an item to put in here"))))))

(fn InteractwithRegister
  (if (Variables|Default|GetIsCarrying)
    (Development|PrintText "My hands are full")
    (elif (Variables|/Game/Level_Workspace/Blueprints/Actors/BP_Register.BP_Register_C|GetIsNPCWaiting (Variables|Default|GetRegisterInstance))
      (CallFunction|OpenRegister)
      (else
        (Development|PrintText "There´s noone here")))))

(fn InteractwithPickUp
  (if (Variables|Default|GetIsCarrying)
    (Development|PrintText "My hands are full")
    (else
      (CallFunction|PickUpItem)
      (Widget|RemovefromParent (Variables|Default|GetInteractPrompt)))))

(fn InteractwithClayStorage
  (bind _asbp_clay_storage (Utilities|Casting|CastToBP_ClayStorage (Variables|Default|GetInteractActor)))
  (if (Variables|Default|GetIsCarrying)
    (if (Variables|Default|GetHasClay)
      (if (< (Variables|/Game/Level_Workspace/Blueprints/Actors/BP_ClayStorage.BP_ClayStorage_C|GetClayAmountStored _asbp_clay_storage) (Variables|/Game/Level_Workspace/Blueprints/Actors/BP_ClayStorage.BP_ClayStorage_C|GetMaximumClayAmount _asbp_clay_storage))
        (CallFunction|DropItem)
        (Actor|DestroyActor (Variables|Default|GetCarriedItem))
        (CallFunction|AddClaytoStorage)
        (Variables|Default|SetCarriedItem (Variables|Default|GetNullActor))
        (else
          (Development|PrintText "This is full.")))
      (else
        (Development|PrintText "My hands are full")))
    (elif (> (Variables|/Game/Level_Workspace/Blueprints/Actors/BP_ClayStorage.BP_ClayStorage_C|GetClayAmountStored _asbp_clay_storage) 0)
      (bind _returnvalue (Game|SpawnActorfromClass "/Game/Crafting_Workspace/BP_Clay.BP_Clay_C" (Transformation|GetWorldTransform (Variables|Default|GetItemPos)) "Undefined" "MultiplyWithRoot" 0 0))
      (Variables|Default|SetHasClay true)
      (Variables|Default|SetIsCarrying true)
      (Variables|Default|SetCarriedItem _returnvalue)
      (Transformation|AttachComponentToComponent (Actor|GetComponentbyClass _returnvalue "/Script/Engine.StaticMeshComponent") (Variables|Default|GetItemPos) "None" "SnapToTarget" "SnapToTarget" "KeepWorld" true)
      (CallFunction|RemoveClayfromStorage)
      (else
        (Development|PrintText "This is empty")))))

(fn OpenUpgradeScreen
  (bind _upgradescreenreference (Variables|Default|GetUpgradeScreenReference))
  (UserInterface|Viewport|AddtoViewport _upgradescreenreference 0)
  (Input|SetInputModeGameandUI (Game|GetPlayerController 0) _upgradescreenreference "DoNotLock" true false)
  (Default|DisplayClayRestockText _upgradescreenreference))

(fn CloseUpgradeScreen
  (Widget|RemovefromParent (Variables|Default|GetUpgradeScreenReference)))