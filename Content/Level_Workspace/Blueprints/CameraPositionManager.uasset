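; Trigger actor that slides the level's CameraActor between a store view and a storage view as the player enters or leaves its Collision component.
; Overlap by a component tagged Player starts movement to CameraPos2 (storage), and end overlap returns it to CameraPos1 (store).
; Each direction runs on a looping 0.01-second timer using VInterpTo at CameraSpeed, cancels the opposite timer, and stops upon reaching its target.
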(event OnComponentBeginOverlap(Collision)
  (params (OverlappedComponent :type Primitive%20Component%20Object%20Reference) (OtherActor :type Actor%20Object%20Reference) (OtherComp :type Primitive%20Component%20Object%20Reference) (OtherBodyIndex :type Integer) (bFromSweep :type Boolean) (SweepResult :type Hit%20Result%20Structure%20%28by%20ref%29))
  (if (Components|ComponentHasTag OtherComp "Player")
    (Utilities|Time|ClearTimerbyFunctionName 0 "MoveToStorePosition")
    (Utilities|Time|SetTimerbyFunctionName 0 "MoveToStoragePosition" 0.01 true)))

(event OnComponentEndOverlap(Collision)
  (params (OverlappedComponent :type Primitive%20Component%20Object%20Reference) (OtherActor :type Actor%20Object%20Reference) (OtherComp :type Primitive%20Component%20Object%20Reference) (OtherBodyIndex :type Integer))
  (if (Components|ComponentHasTag OtherComp "Player")
    (Utilities|Time|ClearTimerbyFunctionName 0 "MoveToStoragePosition")
    (Utilities|Time|SetTimerbyFunctionName 0 "MoveToStorePosition" 0.01 true)))

(event EventBeginPlay
  (bind _returnvalue (Actor|GetActorOfClass "/Script/Engine.CameraActor"))
  (Variables|Default|SetCameraReference _returnvalue))

(fn ConstructionScript)

(fn MovetoStorePosition
  (if (Utilities|Operators|EqualEqual (Transformation|GetWorldLocation (Variables|/Script/Engine.CameraActor|GetCameraComponent (Variables|Default|GetCameraReference))) (Variables|Default|GetCameraPos1) 0.0)
    (Utilities|Time|ClearTimerbyFunctionName 0 "MoveToStorePosition")
    (else
      (Transformation|SetWorldLocation (Variables|/Script/Engine.Actor|GetRootComponent (Variables|Default|GetCameraReference)) (Math|Interpolation|VInterpTo (Transformation|GetWorldLocation (Variables|/Script/Engine.CameraActor|GetCameraComponent (Variables|Default|GetCameraReference))) (Variables|Default|GetCameraPos1) (Utilities|Time|GetWorldDeltaSeconds) (Variables|Default|GetCameraSpeed)) false false))))

(fn MovetoStoragePosition
  (if (Utilities|Operators|EqualEqual (Transformation|GetWorldLocation (Variables|/Script/Engine.CameraActor|GetCameraComponent (Variables|Default|GetCameraReference))) (Variables|Default|GetCameraPos2) 0.0)
    (Utilities|Time|ClearTimerbyFunctionName 0 "MoveToStoragePosition")
    (else
      (Transformation|SetWorldLocation (Variables|/Script/Engine.Actor|GetRootComponent (Variables|Default|GetCameraReference)) (Math|Interpolation|VInterpTo (Transformation|GetWorldLocation (Variables|/Script/Engine.CameraActor|GetCameraComponent (Variables|Default|GetCameraReference))) (Variables|Default|GetCameraPos2) (Utilities|Time|GetWorldDeltaSeconds) (Variables|Default|GetCameraSpeed)) false false))))