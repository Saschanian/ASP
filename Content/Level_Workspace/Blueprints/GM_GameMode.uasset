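; Game mode that runs a day cycle with a recurring rent economy and owns the main HUD.
; Looping timers advance an on-screen clock from 08:00 until closing time, then flag the day over and prompt the player.
; Ending a day resets the clock, charges and multiplies rent on interval days, and refreshes the HUD.
; Money add and subtract helpers guard against overspending; NPC spawning and game over are empty stubs.
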(event EventBeginPlay
  ;[1 1 1] Create Main HUD
  (bind _returnvalue (UserInterface|CreateWidget "/Game/UI_Workspace/Blueprints/MainHUD.MainHUD_C"))
  (bind _output_get (Variables|Default|SetMainHUDInstance _returnvalue))
  (UserInterface|Viewport|AddtoViewport _output_get 0)
  (CallFunction|SetDayandRent))

(fn ConstructionScript)

(fn StartNewDay
  (Variables|Default|SetHasDayStarted true)
  (Utilities|Time|SetTimerbyFunctionName 0 "UpdateTimer" (Variables|Default|GetTimeSpeed) true)
  (Utilities|Time|SetTimerbyFunctionName 0 "SpawnNPCs" (Variables|Default|GetNPCSpawnDelay) true)
  (Default|StopAnim (Variables|Default|GetMainHUDInstance)))

(fn EndDay
  (if (Variables|Default|GetIsDayOver)
    (Variables|/Script/UMG.TextBlock|SetText (Variables|/Game/UI_Workspace/Blueprints/MainHUD.MainHUD_C|GetStartEndDay (Variables|Default|GetMainHUDInstance)) "Press Enter to start the next day")
    (Variables|Default|SetTimerSeconds 0)
    (Variables|Default|SetTimerMinutes 8)
    (Variables|/Script/UMG.TextBlock|SetText (Variables|/Game/UI_Workspace/Blueprints/MainHUD.MainHUD_C|GetClock (Variables|Default|GetMainHUDInstance)) "08:00")
    (Math|Float|IncrementFloat (Variables|Default|GetDayCount)
      (:%20%20
        (CallFunction|PayRent)
        (CallFunction|IncreaseRent)
        (CallFunction|SetDayandRent)
        (Variables|Default|SetIsDayOver false)
        (Variables|Default|SetHasDayStarted false)))))

(fn SpawnNPCs)

(fn UpdateTimer
  ;[1 1 1] Add Minutes And Seconds
  (Math|Integer|IncrementInt (Variables|Default|GetTimerSeconds)
    (:%20%20
      (if (== (Variables|Default|GetTimerSeconds) 60)
        (Variables|Default|SetTimerSeconds 0)
        (Math|Integer|IncrementInt (Variables|Default|GetTimerMinutes)
          (:%20%20
            _)))
      ;[1 1 1] Add 0s To Timer Numbers
      (if (>= (Variables|Default|GetTimerMinutes) 10)
        (if (>= (Variables|Default|GetTimerSeconds) 10)
          (Variables|/Script/UMG.TextBlock|SetText (Variables|/Game/UI_Workspace/Blueprints/MainHUD.MainHUD_C|GetClock (Variables|Default|GetMainHUDInstance)) (Utilities|Text|ToText(String) (Utilities|String|Append (Utilities|String|ToString(Integer) (Variables|Default|GetTimerMinutes)) ":" (Utilities|String|ToString(Integer) (Variables|Default|GetTimerSeconds)))))
          (else
            (Variables|/Script/UMG.TextBlock|SetText (Variables|/Game/UI_Workspace/Blueprints/MainHUD.MainHUD_C|GetClock (Variables|Default|GetMainHUDInstance)) (Utilities|Text|ToText(String) (Utilities|String|Append (Utilities|String|ToString(Integer) (Variables|Default|GetTimerMinutes)) ":" "0" (Utilities|String|ToString(Integer) (Variables|Default|GetTimerSeconds)))))))
        (elif (>= (Variables|Default|GetTimerSeconds) 10)
          (Variables|/Script/UMG.TextBlock|SetText (Variables|/Game/UI_Workspace/Blueprints/MainHUD.MainHUD_C|GetClock (Variables|Default|GetMainHUDInstance)) (Utilities|Text|ToText(String) (Utilities|String|Append "0" (Utilities|String|ToString(Integer) (Variables|Default|GetTimerMinutes)) ":" (Utilities|String|ToString(Integer) (Variables|Default|GetTimerSeconds)))))
          (else
            (Variables|/Script/UMG.TextBlock|SetText (Variables|/Game/UI_Workspace/Blueprints/MainHUD.MainHUD_C|GetClock (Variables|Default|GetMainHUDInstance)) (Utilities|Text|ToText(String) (Utilities|String|Append "0" (Utilities|String|ToString(Integer) (Variables|Default|GetTimerMinutes)) ":" "0" (Utilities|String|ToString(Integer) (Variables|Default|GetTimerSeconds))))))))
      ;[1 1 1] Check if day is over
      (if (== (Variables|Default|GetTimerMinutes) (Variables|Default|GetEndOfDayTime))
        (Utilities|Time|ClearTimerbyFunctionName 0 "UpdateTimer")
        (Utilities|Time|ClearTimerbyFunctionName 0 "SpawnNPCs")
        (Variables|Default|SetIsDayOver true)
        (Default|StartAnim (Variables|Default|GetMainHUDInstance))
        (Variables|/Script/UMG.TextBlock|SetText (Variables|/Game/UI_Workspace/Blueprints/MainHUD.MainHUD_C|GetStartEndDay (Variables|Default|GetMainHUDInstance)) "Press Enter to end the day")))))

(fn SetDayandRent
  (Variables|/Script/UMG.TextBlock|SetText (Variables|/Game/UI_Workspace/Blueprints/MainHUD.MainHUD_C|GetDayCount (Variables|Default|GetMainHUDInstance)) (Utilities|Text|ToText(String) (Utilities|String|Append "Day " (Utilities|String|ToString(Integer) (Class|KismetMathLibrary|ToInt64(Float) (Variables|Default|GetDayCount))))))
  (Variables|/Script/UMG.TextBlock|SetText (Variables|/Game/UI_Workspace/Blueprints/MainHUD.MainHUD_C|GetNextRent (Variables|Default|GetMainHUDInstance)) (Utilities|Text|ToText(String) (Utilities|String|Append "Rent due in: " (Utilities|String|ToString(Integer) (Class|KismetMathLibrary|FFloor64 (- (Variables|Default|GetRentInterval) (.Remainder (Math|Float|Division(WholeandRemainder) (Variables|Default|GetDayCount) (Variables|Default|GetRentInterval)))))) " days")))
  (Variables|/Script/UMG.TextBlock|SetText (Variables|/Game/UI_Workspace/Blueprints/MainHUD.MainHUD_C|GetRentDue (Variables|Default|GetMainHUDInstance)) (Utilities|Text|ToText(String) (Utilities|String|Append "Rent due: " (Utilities|String|ToString(Integer) (Variables|Default|GetRentDue)) "G")))
  (CallFunction|UpdatePlayerMoney))

(fn IncreaseRent
  (bind _rentinterval (Variables|Default|GetRentInterval))
  (if (== (- _rentinterval (.Remainder (Math|Float|Division(WholeandRemainder) (Variables|Default|GetDayCount) (Variables|Default|GetRentInterval)))) _rentinterval)
    (Variables|Default|SetRentDue (* (Variables|Default|GetRentDue) (Variables|Default|GetRentMultiplier)))))

(fn PayRent
  (bind _rentinterval (Variables|Default|GetRentInterval))
  (if (== (- _rentinterval (.Remainder (Math|Float|Division(WholeandRemainder) (Variables|Default|GetDayCount) (Variables|Default|GetRentInterval)))) _rentinterval)
    (bind _output_get (Variables|Default|SetPlayerMoney (- (Variables|Default|GetPlayerMoney) (Variables|Default|GetRentDue))))
    (if (<= _output_get 0)
      (CallFunction|GameOver))))

(fn GameOver)

(fn UpdatePlayerMoney
  (Variables|/Script/UMG.TextBlock|SetText (Variables|/Game/UI_Workspace/Blueprints/MainHUD.MainHUD_C|GetMoney (Variables|Default|GetMainHUDInstance)) (Utilities|Text|ToText(String) (Utilities|String|Append (Utilities|String|ToString(Integer) (Variables|Default|GetPlayerMoney)) "G"))))

(fn AddMoney
  (params (Amount :type Integer))
  (Variables|Default|SetPlayerMoney (+ (Variables|Default|GetPlayerMoney) Amount))
  (CallFunction|UpdatePlayerMoney))

(fn SubtractMoney
  (params (Amount :type Integer))
  (bind _output_get (LocalVariables|SetSubtractMoneySuccess (>= (- (Variables|Default|GetPlayerMoney) Amount) 0)))
  (if _output_get
    (Variables|Default|SetPlayerMoney (- (Variables|Default|GetPlayerMoney) Amount))
    (CallFunction|UpdatePlayerMoney)
    (else
      (Development|PrintText "Not Enough Money")))
  (return (LocalVariables|GetSubtractMoneySuccess)))

(fn FadeScreen
  (if (Variables|Default|GetIsDayOver)
    (Default|FadeScreen (Variables|Default|GetMainHUDInstance))))