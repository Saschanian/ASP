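; BP_CraftingBench is a crafting bench actor with minimal logic, reacting when objects tagged PickUp leave its overlap.
; On end overlap with such an actor, it finds its own Box component and calls Activate on it without a reset.
; Logic to turn a widget toward the player camera exists but is disconnected, and Tick and the construction script are empty.
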(event Collision|EventActorEndOverlap
  (params (OtherActor :type Actor%20Object%20Reference))
  (if (Actor|ActorHasTag OtherActor "PickUp")
    (Components|Activation|Activate (Actor|GetComponentbyClass "/Script/Engine.BoxComponent") false)))

(event EventTick
  (params (DeltaSeconds :type Float%20%28single-precision%29)))

(fn ConstructionScript)