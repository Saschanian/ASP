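; BP_ClayStorage is a clay storage actor that shows how much clay it holds through five components, Clay1 to Clay5.
; Every Tick switches on ClayAmountStored from zero to five, showing lower pieces and hiding only the one just above the count.
; The count of four only hides Clay5, as the nodes that would show Clay1 to Clay4 never run.
; The count is only read here, and the construction script is empty.
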(event EventTick
  (params (DeltaSeconds :type Float%20%28single-precision%29))
  (switch int (Variables|Default|GetClayAmountStored)
    (:0
      (Rendering|SetVisibility (Variables|Default|GetClay1) false true))
    (:1
      (Rendering|SetVisibility (Variables|Default|GetClay2) false true)
      (Rendering|SetVisibility (Variables|Default|GetClay1) true true))
    (:2
      (Rendering|SetVisibility (Variables|Default|GetClay3) false true)
      (Rendering|SetVisibility (Variables|Default|GetClay2) true false)
      (Rendering|SetVisibility (Variables|Default|GetClay1) true false))
    (:3
      (Rendering|SetVisibility (Variables|Default|GetClay4) false true)
      (Rendering|SetVisibility (Variables|Default|GetClay3) true false)
      (Rendering|SetVisibility (Variables|Default|GetClay2) true false)
      (Rendering|SetVisibility (Variables|Default|GetClay1) true false))
    (:4
      (Rendering|SetVisibility (Variables|Default|GetClay5) false true))
    (:5
      (Rendering|SetVisibility (Variables|Default|GetClay5) true true)
      (Rendering|SetVisibility (Variables|Default|GetClay4) true false)
      (Rendering|SetVisibility (Variables|Default|GetClay3) true false)
      (Rendering|SetVisibility (Variables|Default|GetClay2) true false)
      (Rendering|SetVisibility (Variables|Default|GetClay1) true false))))

(fn ConstructionScript)