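; SaveGameManager is meant to persist clay-shop progress: player carry state, money, rent, day, upgrades, clay storage and shop displays.
; BeginPlay creates the "Save" slot if missing and caches references to those sources.
; SaveGame copies live values into the loaded save object and appends storage and display arrays, but never writes it back to the slot.
; LoadGame currently duplicates SaveGame's logic, so it restores nothing to the game.
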(event EventBeginPlay
  ;[1 1 1] Create Save Once
  (bind _returnvalue (SaveGame|DoesSaveGameExist "Save"))
  (if _returnvalue
    _
    (else
      (bind _returnvalue_2 (SaveGame|CreateSaveGameObject "/Game/Level_Workspace/Blueprints/SaveGame.SaveGame_C"))
      (SaveGame|SaveGametoSlot _returnvalue_2 "Save")))
  ;[1 1 1] Get References
  (bind _returnvalue_3 (Actor|GetActorOfClass "/Game/Player_Workspace/Blueprints/BP_PlayerCharacter.BP_PlayerCharacter_C"))
  (Variables|Default|SetPlayerInstance _returnvalue_3)
  (bind _returnvalue_4 (Actor|GetActorOfClass "/Game/Level_Workspace/Blueprints/GM_GameMode.GM_GameMode_C"))
  (Variables|Default|SetGameModeInstance _returnvalue_4)
  (bind _foundwidgets (Widget|GetAllWidgetsOfClass "/Game/UI_Workspace/Blueprints/UpgradeScreen.UpgradeScreen_C" false))
  (Variables|Default|SetUpgradeScreenInstance (Utilities|Array|Get(acopy) _foundwidgets))
  (bind _outactors (Actor|GetAllActorsOfClass "/Game/Level_Workspace/Blueprints/Actors/BP_ClayStorage.BP_ClayStorage_C"))
  (Variables|Default|SetClayStorageInstances _outactors)
  (bind _outactors_2 (Actor|GetAllActorsOfClass "/Game/Level_Workspace/Blueprints/Actors/BP_ShopDisplay.BP_ShopDisplay_C"))
  (Variables|Default|SetShopDisplayInstances _outactors_2))

(fn ConstructionScript)

(fn SaveGame
  (bind _playerinstance (Variables|Default|GetPlayerInstance))
  (bind _gamemodeinstance (Variables|Default|GetGameModeInstance))
  (bind _upgradescreeninstance (Variables|Default|GetUpgradeScreenInstance))
  (bind _returnvalue (SaveGame|LoadGamefromSlot "Save"))
  (bind _assave_game (Utilities|Casting|CastToSaveGame _returnvalue))
  ;[1 1 1] Player Saving
  (Variables|/Game/Level_Workspace/Blueprints/SaveGame.SaveGame_C|SetIsCarrying _assave_game (Variables|/Game/Player_Workspace/Blueprints/BP_PlayerCharacter.BP_PlayerCharacter_C|GetIsCarrying _playerinstance))
  (Variables|/Game/Level_Workspace/Blueprints/SaveGame.SaveGame_C|SetHasClay _assave_game (Variables|/Game/Player_Workspace/Blueprints/BP_PlayerCharacter.BP_PlayerCharacter_C|GetHasClay _playerinstance))
  (Variables|/Game/Level_Workspace/Blueprints/SaveGame.SaveGame_C|SetCarriedItem _assave_game (Variables|/Game/Player_Workspace/Blueprints/BP_PlayerCharacter.BP_PlayerCharacter_C|GetCarriedItem _playerinstance))
  ;[1 1 1] GameMode Saving
  (Variables|/Game/Level_Workspace/Blueprints/SaveGame.SaveGame_C|SetPlayerMoney _assave_game (Variables|/Game/Level_Workspace/Blueprints/GM_GameMode.GM_GameMode_C|GetPlayerMoney _gamemodeinstance))
  (Variables|/Game/Level_Workspace/Blueprints/SaveGame.SaveGame_C|SetRentDue _assave_game (Variables|/Game/Level_Workspace/Blueprints/GM_GameMode.GM_GameMode_C|GetRentDue _gamemodeinstance))
  (Variables|/Game/Level_Workspace/Blueprints/SaveGame.SaveGame_C|SetDayCount _assave_game (Variables|/Game/Level_Workspace/Blueprints/GM_GameMode.GM_GameMode_C|GetDayCount _gamemodeinstance))
  ;[1 1 1] Upgrade Saving
  (Variables|/Game/Level_Workspace/Blueprints/SaveGame.SaveGame_C|SetUpgradeLevel1 _assave_game (Variables|/Game/UI_Workspace/Blueprints/UpgradeScreen.UpgradeScreen_C|GetUpgrade1Level _upgradescreeninstance))
  (Variables|/Game/Level_Workspace/Blueprints/SaveGame.SaveGame_C|SetUpgradeLevel2 _assave_game (Variables|/Game/UI_Workspace/Blueprints/UpgradeScreen.UpgradeScreen_C|GetUpgrade2Level _upgradescreeninstance))
  (Variables|/Game/Level_Workspace/Blueprints/SaveGame.SaveGame_C|SetUpgradeLevel3 _assave_game (Variables|/Game/UI_Workspace/Blueprints/UpgradeScreen.UpgradeScreen_C|GetUpgrade3Level _upgradescreeninstance))
  (Variables|/Game/Level_Workspace/Blueprints/SaveGame.SaveGame_C|SetUpgradeLevel4 _assave_game (Variables|/Game/UI_Workspace/Blueprints/UpgradeScreen.UpgradeScreen_C|GetUpgrade4Level _upgradescreeninstance))
  (Variables|/Game/Level_Workspace/Blueprints/SaveGame.SaveGame_C|SetUpgradeLevel5 _assave_game (Variables|/Game/UI_Workspace/Blueprints/UpgradeScreen.UpgradeScreen_C|GetUpgrade5Level _upgradescreeninstance))
  (Variables|/Game/Level_Workspace/Blueprints/SaveGame.SaveGame_C|SetUpgradeMax1 _assave_game (Variables|/Game/UI_Workspace/Blueprints/UpgradeScreen.UpgradeScreen_C|GetUpgrade1Max _upgradescreeninstance))
  (Variables|/Game/Level_Workspace/Blueprints/SaveGame.SaveGame_C|SetUpgradeMax2 _assave_game (Variables|/Game/UI_Workspace/Blueprints/UpgradeScreen.UpgradeScreen_C|GetUpgrade2Max _upgradescreeninstance))
  (Variables|/Game/Level_Workspace/Blueprints/SaveGame.SaveGame_C|SetUpgradeMax3 _assave_game (Variables|/Game/UI_Workspace/Blueprints/UpgradeScreen.UpgradeScreen_C|GetUpgrade3Max _upgradescreeninstance))
  (Variables|/Game/Level_Workspace/Blueprints/SaveGame.SaveGame_C|SetUpgradeMax4 _assave_game (Variables|/Game/UI_Workspace/Blueprints/UpgradeScreen.UpgradeScreen_C|GetUpgrade4Max _upgradescreeninstance))
  (Variables|/Game/Level_Workspace/Blueprints/SaveGame.SaveGame_C|SetUpgradeMax5 _assave_game (Variables|/Game/UI_Workspace/Blueprints/UpgradeScreen.UpgradeScreen_C|GetUpgrade5Max _upgradescreeninstance))
  (Variables|/Game/Level_Workspace/Blueprints/SaveGame.SaveGame_C|SetUpgradePrice1 _assave_game (Variables|/Game/UI_Workspace/Blueprints/UpgradeScreen.UpgradeScreen_C|GetUpgrade1Price _upgradescreeninstance))
  (Variables|/Game/Level_Workspace/Blueprints/SaveGame.SaveGame_C|SetUpgradePrice2 _assave_game (Variables|/Game/UI_Workspace/Blueprints/UpgradeScreen.UpgradeScreen_C|GetUpgrade2Price _upgradescreeninstance))
  (Variables|/Game/Level_Workspace/Blueprints/SaveGame.SaveGame_C|SetUpgradePrice3 _assave_game (Variables|/Game/UI_Workspace/Blueprints/UpgradeScreen.UpgradeScreen_C|GetUpgrade3Price _upgradescreeninstance))
  (Variables|/Game/Level_Workspace/Blueprints/SaveGame.SaveGame_C|SetUpgradePrice4 _assave_game (Variables|/Game/UI_Workspace/Blueprints/UpgradeScreen.UpgradeScreen_C|GetUpgrade4Price _upgradescreeninstance))
  (Variables|/Game/Level_Workspace/Blueprints/SaveGame.SaveGame_C|SetUpgradePrice5 _assave_game (Variables|/Game/UI_Workspace/Blueprints/UpgradeScreen.UpgradeScreen_C|GetUpgrade5Price _upgradescreeninstance))
  ;[1 1 1] Storage Saving
  (for _array_element (Variables|Default|GetClayStorageInstances)
    (Utilities|Array|Add (Variables|/Game/Level_Workspace/Blueprints/SaveGame.SaveGame_C|GetClayStorages _assave_game) _array_element)
    (Utilities|Array|Add (Variables|/Game/Level_Workspace/Blueprints/SaveGame.SaveGame_C|GetClayAmounts _assave_game) (Variables|/Game/Level_Workspace/Blueprints/Actors/BP_ClayStorage.BP_ClayStorage_C|GetClayAmountStored _array_element)))
  ;[1 1 1] Display Saving
  (for _array_element_2 (Variables|Default|GetShopDisplayInstances)
    (Utilities|Array|Add (Variables|/Game/Level_Workspace/Blueprints/SaveGame.SaveGame_C|GetShopDisplays _assave_game) _array_element_2)
    (Utilities|Array|Add (Variables|/Game/Level_Workspace/Blueprints/SaveGame.SaveGame_C|GetShopDisplayItems _assave_game) (Variables|/Game/Level_Workspace/Blueprints/Actors/BP_ShopDisplay.BP_ShopDisplay_C|GetHeldItem _array_element_2))))

(fn LoadGame
  (bind _playerinstance (Variables|Default|GetPlayerInstance))
  (bind _gamemodeinstance (Variables|Default|GetGameModeInstance))
  (bind _upgradescreeninstance (Variables|Default|GetUpgradeScreenInstance))
  (bind _returnvalue (SaveGame|LoadGamefromSlot "Save"))
  (bind _assave_game (Utilities|Casting|CastToSaveGame _returnvalue))
  ;[1 1 1] Player Saving
  (Variables|/Game/Level_Workspace/Blueprints/SaveGame.SaveGame_C|SetIsCarrying _assave_game (Variables|/Game/Player_Workspace/Blueprints/BP_PlayerCharacter.BP_PlayerCharacter_C|GetIsCarrying _playerinstance))
  (Variables|/Game/Level_Workspace/Blueprints/SaveGame.SaveGame_C|SetHasClay _assave_game (Variables|/Game/Player_Workspace/Blueprints/BP_PlayerCharacter.BP_PlayerCharacter_C|GetHasClay _playerinstance))
  (Variables|/Game/Level_Workspace/Blueprints/SaveGame.SaveGame_C|SetCarriedItem _assave_game (Variables|/Game/Player_Workspace/Blueprints/BP_PlayerCharacter.BP_PlayerCharacter_C|GetCarriedItem _playerinstance))
  ;[1 1 1] GameMode Saving
  (Variables|/Game/Level_Workspace/Blueprints/SaveGame.SaveGame_C|SetPlayerMoney _assave_game (Variables|/Game/Level_Workspace/Blueprints/GM_GameMode.GM_GameMode_C|GetPlayerMoney _gamemodeinstance))
  (Variables|/Game/Level_Workspace/Blueprints/SaveGame.SaveGame_C|SetRentDue _assave_game (Variables|/Game/Level_Workspace/Blueprints/GM_GameMode.GM_GameMode_C|GetRentDue _gamemodeinstance))
  (Variables|/Game/Level_Workspace/Blueprints/SaveGame.SaveGame_C|SetDayCount _assave_game (Variables|/Game/Level_Workspace/Blueprints/GM_GameMode.GM_GameMode_C|GetDayCount _gamemodeinstance))
  ;[1 1 1] Upgrade Saving
  (Variables|/Game/Level_Workspace/Blueprints/SaveGame.SaveGame_C|SetUpgradeLevel1 _assave_game (Variables|/Game/UI_Workspace/Blueprints/UpgradeScreen.UpgradeScreen_C|GetUpgrade1Level _upgradescreeninstance))
  (Variables|/Game/Level_Workspace/Blueprints/SaveGame.SaveGame_C|SetUpgradeLevel2 _assave_game (Variables|/Game/UI_Workspace/Blueprints/UpgradeScreen.UpgradeScreen_C|GetUpgrade2Level _upgradescreeninstance))
  (Variables|/Game/Level_Workspace/Blueprints/SaveGame.SaveGame_C|SetUpgradeLevel3 _assave_game (Variables|/Game/UI_Workspace/Blueprints/UpgradeScreen.UpgradeScreen_C|GetUpgrade3Level _upgradescreeninstance))
  (Variables|/Game/Level_Workspace/Blueprints/SaveGame.SaveGame_C|SetUpgradeLevel4 _assave_game (Variables|/Game/UI_Workspace/Blueprints/UpgradeScreen.UpgradeScreen_C|GetUpgrade4Level _upgradescreeninstance))
  (Variables|/Game/Level_Workspace/Blueprints/SaveGame.SaveGame_C|SetUpgradeLevel5 _assave_game (Variables|/Game/UI_Workspace/Blueprints/UpgradeScreen.UpgradeScreen_C|GetUpgrade5Level _upgradescreeninstance))
  (Variables|/Game/Level_Workspace/Blueprints/SaveGame.SaveGame_C|SetUpgradeMax1 _assave_game (Variables|/Game/UI_Workspace/Blueprints/UpgradeScreen.UpgradeScreen_C|GetUpgrade1Max _upgradescreeninstance))
  (Variables|/Game/Level_Workspace/Blueprints/SaveGame.SaveGame_C|SetUpgradeMax2 _assave_game (Variables|/Game/UI_Workspace/Blueprints/UpgradeScreen.UpgradeScreen_C|GetUpgrade2Max _upgradescreeninstance))
  (Variables|/Game/Level_Workspace/Blueprints/SaveGame.SaveGame_C|SetUpgradeMax3 _assave_game (Variables|/Game/UI_Workspace/Blueprints/UpgradeScreen.UpgradeScreen_C|GetUpgrade3Max _upgradescreeninstance))
  (Variables|/Game/Level_Workspace/Blueprints/SaveGame.SaveGame_C|SetUpgradeMax4 _assave_game (Variables|/Game/UI_Workspace/Blueprints/UpgradeScreen.UpgradeScreen_C|GetUpgrade4Max _upgradescreeninstance))
  (Variables|/Game/Level_Workspace/Blueprints/SaveGame.SaveGame_C|SetUpgradeMax5 _assave_game (Variables|/Game/UI_Workspace/Blueprints/UpgradeScreen.UpgradeScreen_C|GetUpgrade5Max _upgradescreeninstance))
  (Variables|/Game/Level_Workspace/Blueprints/SaveGame.SaveGame_C|SetUpgradePrice1 _assave_game (Variables|/Game/UI_Workspace/Blueprints/UpgradeScreen.UpgradeScreen_C|GetUpgrade1Price _upgradescreeninstance))
  (Variables|/Game/Level_Workspace/Blueprints/SaveGame.SaveGame_C|SetUpgradePrice2 _assave_game (Variables|/Game/UI_Workspace/Blueprints/UpgradeScreen.UpgradeScreen_C|GetUpgrade2Price _upgradescreeninstance))
  (Variables|/Game/Level_Workspace/Blueprints/SaveGame.SaveGame_C|SetUpgradePrice3 _assave_game (Variables|/Game/UI_Workspace/Blueprints/UpgradeScreen.UpgradeScreen_C|GetUpgrade3Price _upgradescreeninstance))
  (Variables|/Game/Level_Workspace/Blueprints/SaveGame.SaveGame_C|SetUpgradePrice4 _assave_game (Variables|/Game/UI_Workspace/Blueprints/UpgradeScreen.UpgradeScreen_C|GetUpgrade4Price _upgradescreeninstance))
  (Variables|/Game/Level_Workspace/Blueprints/SaveGame.SaveGame_C|SetUpgradePrice5 _assave_game (Variables|/Game/UI_Workspace/Blueprints/UpgradeScreen.UpgradeScreen_C|GetUpgrade5Price _upgradescreeninstance))
  ;[1 1 1] Storage Saving
  (for _array_element (Variables|Default|GetClayStorageInstances)
    (Utilities|Array|Add (Variables|/Game/Level_Workspace/Blueprints/SaveGame.SaveGame_C|GetClayStorages _assave_game) _array_element)
    (Utilities|Array|Add (Variables|/Game/Level_Workspace/Blueprints/SaveGame.SaveGame_C|GetClayAmounts _assave_game) (Variables|/Game/Level_Workspace/Blueprints/Actors/BP_ClayStorage.BP_ClayStorage_C|GetClayAmountStored _array_element)))
  ;[1 1 1] Display Saving
  (for _array_element_2 (Variables|Default|GetShopDisplayInstances)
    (Utilities|Array|Add (Variables|/Game/Level_Workspace/Blueprints/SaveGame.SaveGame_C|GetShopDisplays _assave_game) _array_element_2)
    (Utilities|Array|Add (Variables|/Game/Level_Workspace/Blueprints/SaveGame.SaveGame_C|GetShopDisplayItems _assave_game) (Variables|/Game/Level_Workspace/Blueprints/Actors/BP_ShopDisplay.BP_ShopDisplay_C|GetHeldItem _array_element_2))))